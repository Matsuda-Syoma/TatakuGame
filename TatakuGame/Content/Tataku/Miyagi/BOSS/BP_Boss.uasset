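; Boss actor that attacks the player at close range and is destroyed when its HP runs out.
; Each tick, Attack_system counts frames while the player is within range; past a threshold it briefly shows and enables the attack collider.
; Leaving range resets the counter and hides the attack.
; Overlapping the attack launches the player along a fixed world vector without applying damage.
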(event `self.ReceiveBeginPlay`
  ;[1 0 0] BeginPlay
  (set `self.SP` (make `/Game/Tataku/Miyagi/ST_CharaSpec` (`self.HP`)))
  (`PrimitiveComponent.SetCollisionEnabled` (`self.S_attack`) "NoCollision"))

(event `self.ReceiveTick`
  (params (DeltaSeconds :type "Float (single-precision)"))
  (bind _s_attack (`self.S_attack`))
  ;[1 0.9749 0] Tick
  (bind _length (`self.VectorLength` (`GameplayStatics.GetPlayerPawn` 0))) ; 距離を図る関数
  (if (< _length 300.0)
    (bind _result (`/Engine/EditorBlueprintResources/StandardMacros.IncrementInt` (`self.S_Rate`)) ; 距離が近いならレートを動かす
      (:`  `
        (bind _output_get (set `self.S_Rate` _result))
        (if (> _output_get (`self.S_Attack_Timing`))
          (`PrimitiveComponent.SetCollisionEnabled` _s_attack "QueryOnly")
          (`SceneComponent.SetVisibility` _s_attack true false)
          (`KismetSystemLibrary.Delay` 0.3)
          (set `self.S_Rate` 0)
          (else
            (`PrimitiveComponent.SetCollisionEnabled` _s_attack "NoCollision" :!label _label)
            (`SceneComponent.SetVisibility` _s_attack false false)))))
    (else
      (set `self.S_Rate` 0) ; 攻撃反応速度の初期化
      (goto _label))))

(event `self.ReceiveAnyDamage`
  (params (Damage :type "Float (single-precision)") (DamageType :type "DamageType Object Reference") (InstigatedBy :type "Controller Object Reference") (DamageCauser :type "Actor Object Reference"))
  (bind _sp_hp (break `/Game/Tataku/Miyagi/ST_CharaSpec` (`self.SP`)))
  ;[1 1 1] ダメージ処理
  (bind _output_get (set `self.SP` (make `/Game/Tataku/Miyagi/ST_CharaSpec` (- _sp_hp Damage))))
  (`KismetSystemLibrary.PrintString` (`KismetStringLibrary.Conv_DoubleToString` _sp_hp))
  (if (< (break `/Game/Tataku/Miyagi/ST_CharaSpec` _output_get) 1.0)
    (`self.K2_DestroyActor`)))

(event `self.S_attack.OnComponentBeginOverlap`
  (params (OverlappedComponent :type "PrimitiveComponent Object Reference") (OtherActor :type "Actor Object Reference") (OtherComp :type "PrimitiveComponent Object Reference") (OtherBodyIndex :type Integer) (bFromSweep :type Boolean) (SweepResult :type "HitResult Structure (by ref)"))
  ;[1 1 1] Attack_Collision
  (bind _asbp_player_ma (cast `/Game/Tataku/Matsuda/Player/BP_Player_Ma` OtherActor))
  (`self.LaunchCharacter` _asbp_player_ma (1000.0 0.0 100.0) false false))

(fn `UserConstructionScript`)

(fn `VectorLength`
  (params (Actor :type "Actor Object Reference"))
  (returns (Length :type "Float (double-precision)"))
  (return (`KismetMathLibrary.VSize` (- (`self.K2_GetActorLocation`) (`self.K2_GetActorLocation` Actor)))))