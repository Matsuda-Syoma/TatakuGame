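; Side-view player character that moves along X, jumps, dashes and performs a charged attack through Enhanced Input.
; Double-tapping a direction within a short retriggerable window calls Boost, which switches to Falling and overrides X velocity.
; Holding attack builds capped Power with a Niagara effect, and release passes half to the Weapon component added at BeginPlay.
; Helper functions flip facing by input and lengthen the camera arm with height; CoolTimeFunc is empty.
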(event `self.ReceiveBeginPlay`
  (bind _asplayer_controller (cast `PlayerController` (`self.GetController`)))
  (`EnhancedInputSubsystemInterface.AddMappingContext` (pcsubsystem `EnhancedInputLocalPlayerSubsystem` _asplayer_controller) "/Game/Tataku/Matsuda/Input/IMC_Player_Ma.IMC_Player_Ma" 0 (struct))
  (bind _returnvalue (`|AddComponentByClass` "/Game/Tataku/Matsuda/Player/NewBlueprint.NewBlueprint_C"))
  (set `self.Weapon` _returnvalue)
  (`KismetSystemLibrary.K2_SetTimerDelegate` (`|CreateDelegate` :!event `SetRotation`) 0.016667 true)
  (`KismetSystemLibrary.K2_SetTimerDelegate` (`|CreateDelegate` :!event `SetCameraLocation`) 0.016667 true)
  (`KismetSystemLibrary.K2_SetTimerDelegate` (`|CreateDelegate` :!event `CoolTimeFunc`) 0.016667 true)
  (set `self.BaseLocation` (`self.K2_GetActorLocation`)))

(event `EnhancedInput|/Game/Tataku/Matsuda/Input/IA_Move`
  (params (ActionValue :type "Float (double-precision)") (ElapsedSeconds :type "Float (double-precision)") (TriggeredSeconds :type "Float (double-precision)") (InputAction :type "InputAction Object Reference" :default "/Game/Tataku/Matsuda/Input/IA_Move.IA_Move"))
  (:`Triggered`
    (`self.AddMovementInput` (`KismetMathLibrary.MakeVector` ActionValue))
    (`/Engine/EditorBlueprintResources/StandardMacros.DoOnce` false :!label _label
      (:`Completed`
        (`|ExecutionSequence`
          (:`then_0`
            (if (> ActionValue 0.0)
              (`/Engine/EditorBlueprintResources/StandardMacros.IncrementInt` (`self.Left`)
                (:`  `
                  (set `self.Right` 0)
                  (if (>= (`self.Left`) 2)
                    (`self.Boost` 2500.0)
                    (set `self.Left` 0)
                    (set `self.Right` 0))))
              (else
                (`/Engine/EditorBlueprintResources/StandardMacros.IncrementInt` (`self.Right`)
                  (:`  `
                    (set `self.Left` 0)
                    (if (>= (`self.Right`) 2)
                      (`self.Boost` -2500.0)
                      (set `self.Left` 0)
                      (set `self.Right` 0)))))))
          (:`then_1`
            (`KismetSystemLibrary.RetriggerableDelay` 0.2)
            (set `self.Left` 0)
            (set `self.Right` 0))))))
  (:`Canceled`
    (goto _label :!via `Reset`))
  (:`Completed`
    (goto _label :!via `Reset`)))

(event `EnhancedInput|/Game/Tataku/Matsuda/Input/IA_Jump`
  (params (ActionValue :type Boolean) (ElapsedSeconds :type "Float (double-precision)") (TriggeredSeconds :type "Float (double-precision)") (InputAction :type "InputAction Object Reference" :default "/Game/Tataku/Matsuda/Input/IA_Jump.IA_Jump"))
  (:`Started`
    (`self.Jump`)))

(event `EnhancedInput|/Game/Tataku/Matsuda/Input/IA_Attack`
  (params (ActionValue :type Boolean) (ElapsedSeconds :type "Float (double-precision)") (TriggeredSeconds :type "Float (double-precision)") (InputAction :type "InputAction Object Reference" :default "/Game/Tataku/Matsuda/Input/IA_Attack.IA_Attack"))
  (:`Triggered`
    (if (> (`self.MaxPower`) (`self.Power`))
      (`/Engine/EditorBlueprintResources/StandardMacros.IncrementInt` (`self.Power`))))
  (:`Started`
    (`ActorComponent.SetActive` (`self.NewNiagaraSystem1`) true false))
  (:`Canceled`
    (`ActorComponent.SetActive` (`self.NewNiagaraSystem1`) false false))
  (:`Completed`
    (`/Game/Tataku/Matsuda/Player/NewBlueprint.Attack` (`self.Weapon`) (`KismetMathLibrary.Conv_IntToDouble` (/ (`self.Power`) 2)))
    (set `self.Power` 0)
    (`ActorComponent.SetActive` (`self.NewNiagaraSystem1`) false false)))

(fn `Boost`
  (params (X :type "Float (double-precision)"))
  (bind (_returnvalue_x _returnvalue_y _returnvalue_z) (`KismetMathLibrary.BreakVector` (`self.GetVelocity`)))
  (`CharacterMovementComponent.SetMovementMode` (`self.CharacterMovement`) "MOVE_Falling" 0)
  (set `MovementComponent.Velocity` (`KismetMathLibrary.MakeVector` X _returnvalue_y _returnvalue_z) (`self.CharacterMovement`)))

(fn `CoolTimeFunc`)

(fn `SetCameraLocation`
  (set `SpringArmComponent.TargetArmLength` (+ (.z (- (`self.K2_GetActorLocation`) (`self.BaseLocation`))) 900.0) (`self.SpringArm`)))

(fn `SetRotation`
  (if (< (`|GetInputActionValue`) -0.01)
    (`self.K2_SetActorRotation` (struct :`Yaw` 180.0)) ; 左に向く
    (elif (> (`|GetInputActionValue`) 0.01)
      (`self.K2_SetActorRotation` (struct)) ; 右に向く
    )))

(fn `UserConstructionScript`)